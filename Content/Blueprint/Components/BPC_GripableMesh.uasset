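; BPC_GripableMesh is a component that makes an object grippable by an interactor's hand and relays interaction events.
; Grip stores the gripping hand and fires ONGrip with the interactor, while Drop resets the hand value and fires ONDrop.
; Hover and UnHover fire dispatchers with crossed names: Hover calls OnUnHover and UnHover calls OnHover.
; GetStatus returns the current GrippingHand value.
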(event `/Game/Blueprint/Interfaces/BPI_GripInterface.Grip`
  (params (Interactor :type "SphereComponent Object Reference") (hand :type "/Game/Blueprint/Data/Enum_HandType Enum" :default "NewEnumerator0"))
  (set `self.GrippingHand` hand)
  (`self.ONGrip` Interactor))

(event `/Game/Blueprint/Interfaces/BPI_GripInterface.Drop`
  (set `self.GrippingHand` "NewEnumerator2")
  (`self.ONDrop`))

(event `/Game/Blueprint/Interfaces/BPI_GripInterface.UnHover`
  (`self.OnHover`))

(event `/Game/Blueprint/Interfaces/BPI_GripInterface.Hover`
  (`self.OnUnHover`))

(fn `GetStatus`
  (returns (GripBY :type "/Game/Blueprint/Data/Enum_HandType Enum"))
  (return (`self.GrippingHand`)))
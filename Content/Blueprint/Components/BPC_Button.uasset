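; VR push-button component that a VRPawn's grab collision physically presses, working as either a toggle or a non-toggle button.
; Overlap starts tick tracking of the hand's depth in button space, moving the button along local Z within a clamped travel.
; Crossing the toggle depth updates state with a minimum interval between changes, calls ButtonPressed and swaps green/red material.
; When overlap ends, it interpolates back toward its starting position.
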(event `self.ReceiveTick`
  (params (DeltaSeconds :type "Float (single-precision)"))
  (`|ExecutionSequence`
    (:`then_0`
      (if (`self.isEnabled`)
        (`self.UpdateButtonLocation`)
        (elif (not (`self.Lerping`))
          (set `self.FocusActor` null)
          (set `self.FocusedComponent` null)
          (set `self.Lerping` true))))
    (:`then_1`
      (`self.LerpReturnMoveButton`)
      (`self.UpdateButtonStateFndColor`))))

(event `self.ReceiveBeginPlay`
  (remove `self.OnComponentBeginOverlap` (`|CreateDelegate` :!event `ComponentBeginOverlap`))
  (add `self.OnComponentEndOverlap` (`|CreateDelegate` :!event `ComponentEndOverlap`))
  (set `self.StartupTransform` (`self.GetRelativeTransform`)))

(event `ComponentBeginOverlap` :!signature `self.OnComponentBeginOverlap`
  (params (OverlappedComponent :type "PrimitiveComponent Object Reference") (OtherActor :type "Actor Object Reference") (OtherComp :type "PrimitiveComponent Object Reference") (OtherBodyIndex :type Integer) (bFromSweep :type Boolean) (SweepResult :type "HitResult Structure (by ref)"))
  (bind _asvrpawn (cast `/Game/Blueprint/Game/VRPawn` OtherActor))
  (bind _output_get (set `self.FocusActor` _asvrpawn))
  (bind _leftgrapcollision (`/Game/Blueprint/Game/VRPawn.LeftGrapCollision` _output_get))
  (bind _rightgrapcollision (`/Game/Blueprint/Game/VRPawn.RightGrapCollision` _output_get))
  (bind _returnvalue (== _rightgrapcollision OtherComp))
  (if (or (== OtherComp _leftgrapcollision) _returnvalue)
    (bind _output_get_2 (set `self.FocusedComponent` (select `bool` _returnvalue :`false` _leftgrapcollision :`true` _rightgrapcollision)))
    (`self.StartButtonTransforming` _output_get_2)))

(event `ComponentEndOverlap` :!signature `self.OnComponentEndOverlap`
  (params (OverlappedComponent :type "PrimitiveComponent Object Reference") (OtherActor :type "Actor Object Reference") (OtherComp :type "PrimitiveComponent Object Reference") (OtherBodyIndex :type Integer))
  (if (`self.isEnabled`)
    (if (== OtherActor (`self.FocusActor`))
      (set `self.FocusActor` null)
      (set `self.FocusedComponent` null)
      (set `self.isEnabled` false))))

(fn `ChekButtonPressed`
  (params (State :type Boolean))
  (returns (succes :type Boolean))
  (bind _toggledthistouch (`self.ToggledThisTouch`))
  (if (>= (`KismetMathLibrary.GetTotalSeconds` (- (`KismetMathLibrary.Now`) (`self.LastToggleTime`))) (`self.MaxTimeBetweenToggle`))
    (if (`self.toggligButton`)
      (if _toggledthistouch
        (set `self.ToggledThisTouch` (not _toggledthistouch))
        (bind _output_get (set `self.ButtonState` (not (`self.ButtonState`))))
        (`self.ButtonPressed` _output_get)
        (set `self.LastToggleTime` (`KismetMathLibrary.Now`))
        (return _output_get)
        (else
          (set `self.ToggledThisTouch` (not (`self.ToggledThisTouch`)))))
      (else
        (bind _output_get_2 (set `self.ButtonState` State))
        (`self.ButtonPressed` _output_get_2)
        (set `self.LastToggleTime` (`KismetMathLibrary.Now`))))
    (else
      (return false))))

(fn `GEtCurrentTransform`
  (returns (CurrentTransform :type "Transform Structure"))
  (`self.FocusActor`
    (:`then`
      (return (`KismetMathLibrary.ComposeTransforms` (`self.StartupTransform`) (`self.K2_GetComponentToWorld` (`self.GetAttachParent`)))))
    (:`else`
      (return (`self.StartupTransform`)))))

(fn `LerpReturnMoveButton`
  (bind _startuptransform_location (`KismetMathLibrary.BreakTransform` (`self.StartupTransform`)))
  (bind _returnvalue (`KismetMathLibrary.VInterpTo_Constant` (`self.RelativeLocation`) _startuptransform_location (`GameplayStatics.GetWorldDeltaSeconds`) (`self.ReturnSpeed`)))
  (if (`self.Lerping`)
    (`self.K2_SetRelativeLocation` _returnvalue)
    (if (== _returnvalue (0.0 0.0 0.0))
      (set `self.Lerping` false)
      (`self.SetComponentTickEnabled` false))))

(fn `Set button color`
  (params (`State ` :type Boolean))
  (if `State `
    (`self.SetMaterial` 0 "/Game/Meshes/Materials/M_ColorGreen.M_ColorGreen")
    (else
      (`self.SetMaterial` 0 "/Game/Meshes/Materials/M_ColorRed.M_ColorRed"))))

(fn `StartButtonTransforming`
  (params (Component :type "SphereComponent Object Reference"))
  (bind _currenttransform (`self.GEtCurrentTransform`))
  (bind (_returnvalue_x _returnvalue_y _returnvalue_z) (`KismetMathLibrary.BreakVector` (`KismetMathLibrary.InverseTransformLocation` _currenttransform (`self.K2_GetComponentLocation`))))
  (bind (_returnvalue_x_2 _returnvalue_y_2 _returnvalue_z_2) (`KismetMathLibrary.BreakVector` (`KismetMathLibrary.InverseTransformLocation` _currenttransform (`self.K2_GetComponentLocation` Component))))
  (set `self.StartupLocalZ` _returnvalue_z_2)
  (set `self.StartupComponentZ` _returnvalue_z)
  (`self.SetComponentTickEnabled` true)
  (set `self.Lerping` false)
  (set `self.ToggledThisTouch` true)
  (set `self.isEnabled` true))

(fn `UpdateButtonLocation`
  (bind (_returnvalue_x _returnvalue_y _returnvalue_z) (`KismetMathLibrary.BreakVector` (`KismetMathLibrary.InverseTransformLocation` (`self.GEtCurrentTransform`) (`self.K2_GetComponentLocation` (`self.FocusedComponent`)))))
  (bind _returnvalue (`KismetMathLibrary.FClamp` (- (`self.StartupLocalZ`) _returnvalue_z) 0.0 (`self.MaxMoveDistants`)))
  (if (> _returnvalue 0.0)
    (`self.K2_SetRelativeLocation` (`KismetMathLibrary.TransformLocation` (`self.StartupTransform`) (`KismetMathLibrary.MakeVector` 0.0 0.0 (`KismetMathLibrary.FClamp` (+ (`self.StartupComponentZ`) (* _returnvalue -1.0)) (* (`self.MaxMoveDistants`) -1.0)))))))

(fn `UpdateButtonStateFndColor`
  (bind (_returnvalue_x _returnvalue_y _returnvalue_z) (`KismetMathLibrary.BreakVector` (`KismetMathLibrary.InverseTransformLocation` (`self.StartupTransform`) (`self.RelativeLocation`))))
  (bind _returnvalue (!= (<= _returnvalue_z (+ (* (`self.TogglingZoneHeiting`) -1.0) 0.001)) (`self.ButtonState`)))
  (if _returnvalue
    (`/Engine/EditorBlueprintResources/StandardMacros.DoOnce` false :!label _label
      (:`Completed`
        (if (`self.toggligButton`)
          (if (`self.ToggledThisTouch`)
            (bind _succes (`self.ChekButtonPressed` (`self.ButtonState`)))
            (`self.Set button color` _succes))
          (else
            (bind _output_get (set `self.ButtonState` _returnvalue))
            (`self.ChekButtonPressed` _output_get)
            (`self.Set button color` _output_get)))))
    (else
      (goto _label :!via `Reset`))))
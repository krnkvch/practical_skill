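; BP_WidgetBand1 is an actor that holds a widget, revealed through look-at events.
; BeginPlay hides the Widget component, and the Lookat event makes it visible.
; LookAvay also sets it visible, so nothing in this graph hides the widget again after it is first shown.
; Overlap and Tick are disabled, and the construction script only calls its parent.
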(event `self.ReceiveBeginPlay`
  (`parent.ReceiveBeginPlay`)
  (`SceneComponent.SetVisibility` (`self.Widget`) false false))

(event `/Game/Blueprint/Interfaces/BP_LookInterface.LookAt`
  (`SceneComponent.SetVisibility` (`self.Widget`) true false))

(event `/Game/Blueprint/Interfaces/BP_LookInterface.LookAvay`
  (`SceneComponent.SetVisibility` (`self.Widget`) true false))

(fn `UserConstructionScript`
  (`parent.UserConstructionScript`))
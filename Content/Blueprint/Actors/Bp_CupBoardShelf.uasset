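; A cupboard shelf actor that slides along its local X axis when gripped by its handle, like a drawer.
; Handle grip and drop events set or clear the stored interactor, while hover events swap the handle material between green and gray.
; Each tick, the gripping interactor's position is converted to actor space, offset by the handle's relative location, and clamped up to MaxDistance to move the Axes component.
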(event `self.ReceiveBeginPlay`
  (add `/Game/Blueprint/Components/BPC_GripableMesh.ONGrip` (`self.SelfHandle`) (`|CreateDelegate` :!event `EventOnGRip`))
  (add `/Game/Blueprint/Components/BPC_GripableMesh.ONDrop` (`self.SelfHandle`) (`|CreateDelegate` :!event `EventOnDrop`))
  (add `/Game/Blueprint/Components/BPC_GripableMesh.OnHover` (`self.SelfHandle`) (`|CreateDelegate` :!event `EventOnHover`))
  (add `/Game/Blueprint/Components/BPC_GripableMesh.OnUnHover` (`self.SelfHandle`) (`|CreateDelegate` :!event `EventOnUnHover`)))

(event `EventOnGRip`
  (params (Interactor :type "SphereComponent Object Reference"))
  (set `self.Interactor` Interactor))

(event `EventOnDrop`
  (set `self.Interactor` null))

(event `self.ReceiveTick`
  (params (DeltaSeconds :type "Float (single-precision)"))
  (`self.Interactor`
    (:`then`
      (`SceneComponent.K2_SetRelativeLocation` (`self.Axes`) (`KismetMathLibrary.MakeVector` (`KismetMathLibrary.FClamp` (`self.CalculateLocation`) 0.0 (`self.MaxDistance`))) false false))
    (:`else`)))

(event `EventOnHover`
  (`PrimitiveComponent.SetMaterial` (`self.SelfHandle`) 0 "/Game/Meshes/Materials/M_ColorGreen.M_ColorGreen"))

(event `EventOnUnHover`
  (`PrimitiveComponent.SetMaterial` (`self.SelfHandle`) 0 "/Game/Meshes/Materials/M_ColorGray.M_ColorGray"))

(fn `CalculateLocation`
  (returns (Value :type "Float (double-precision)"))
  (bind _interactor (`self.Interactor`)
    (:`then`
      (bind _returnvalue_x (`KismetMathLibrary.BreakVector` (- (`KismetMathLibrary.InverseTransformLocation` (`self.GetTransform`) (`SceneComponent.K2_GetComponentLocation` _interactor)) (`SceneComponent.RelativeLocation` (`self.SelfHandle`)))))
      (return _returnvalue_x))
    (:`else`)))

(fn `UserConstructionScript`)
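; Showcase actor that displays a configurable static mesh paired with a BP_Commentary_Box child actor.
; Construction script applies the mesh and caches the commentary box; the step copying Lines into it is disconnected.
; Lookat and LookAvay events switch the box on and off, and GetType reports a fixed enum value.
; Tick holds a mesh yaw spin behind a Gate that starts closed and is never opened.
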(event `self.ReceiveTick`
  (params (DeltaSeconds :type "Float (single-precision)"))
  (`/Engine/EditorBlueprintResources/StandardMacros.Gate` true
    (:`Exit`
      (`SceneComponent.K2_AddLocalRotation` (`self.StaticMesh`) (struct :`Yaw` 1.0) false false))))

(event `/Game/Blueprint/Interfaces/BP_LookInterface.LookAt`
  (`/Game/Blueprint/Interfaces/BPI_ElectricSwitchable.TurrON` (`self.TipActorReference`)))

(event `/Game/Blueprint/Interfaces/BP_LookInterface.LookAvay`
  (`/Game/Blueprint/Interfaces/BPI_ElectricSwitchable.TurrOFF` (`self.TipActorReference`)))

(fn `GetType`
  (returns (`Type of interact` :type "/Game/Blueprint/Data/Enum_InteractType Enum"))
  (return "NewEnumerator0"))

(fn `UserConstructionScript`
  (`StaticMeshComponent.SetStaticMesh` (`self.StaticMesh`) (`self.Mesh`))
  (bind _asbp_commentary_box (cast `/Game/Assets/Blueprints/BP_Commentary_Box` (`ChildActorComponent.ChildActor` (`self.BP_Commentary_Box`))))
  (bind _output_get (set `self.TipActorReference` _asbp_commentary_box)))
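; BP_PickupBase is a base pickup actor that an interactor can grip and drop.
; The construction script applies the Mesh variable to its static mesh component.
; Grip turns off physics and attaches the mesh component, not the actor, to the Interactor, keeping world location and rotation.
; Drop re-enables physics simulation and detaches the mesh.
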(event `/Game/Blueprint/Interfaces/BPI_GripInterface.Grip`
  (params (Interactor :type "SphereComponent Object Reference"))
  (`PrimitiveComponent.SetSimulatePhysics` (`self.StaticMesh`) false)
  (`SceneComponent.K2_AttachToComponent` (`self.StaticMesh`) Interactor "None" "KeepWorld" "KeepWorld" "KeepRelative" true))

(event `/Game/Blueprint/Interfaces/BPI_GripInterface.Drop`
  (`PrimitiveComponent.SetSimulatePhysics` (`self.StaticMesh`) true)
  (`SceneComponent.K2_DetachFromComponent` (`self.StaticMesh`) "KeepRelative" "KeepRelative" "KeepRelative" true))

(fn `UserConstructionScript`
  (`StaticMeshComponent.SetStaticMesh` (`self.StaticMesh`) (`self.Mesh`)))
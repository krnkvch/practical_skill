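; Drivable VR tractor that the player enters and exits with buttons, attaching the VRPawn to the cab and locking its movement.
; Four child-actor levers, bound through BPI_Lever, set left and right drive inputs and two bucket target angles.
; Each tick applies tank-style forces at either side of the physics-driven TractorTires, with input-scaled linear damping, yaw damping and sideways velocity adjustment.
; Bucket and arm pitches interpolate toward their lever targets.
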(event `self.ReceiveBeginPlay`
  (add `/Game/Blueprint/Components/BPC_Button.ButtonPressed` (`self.BPC_ButtonEnter`) (`|CreateDelegate` :!event `ButtonEnterPresset`))
  (add `/Game/Blueprint/Components/BPC_Button.ButtonPressed` (`self.BPC_ButtonExit`) (`|CreateDelegate` :!event `ButtonExitPresset`))
  (bind _asbpi_lever (cast `/Game/Blueprint/Actors/BPI_Lever` (`ChildActorComponent.ChildActor` (`self.BP_LeverLeft`))))
  (add `/Game/Blueprint/Actors/BPI_Lever.UpdateLever` _asbpi_lever (`|CreateDelegate` :!event `UpdateLeftLever`))
  (bind _asbpi_lever_2 (cast `/Game/Blueprint/Actors/BPI_Lever` (`ChildActorComponent.ChildActor` (`self.BP_LeverRight`))))
  (add `/Game/Blueprint/Actors/BPI_Lever.UpdateLever` _asbpi_lever_2 (`|CreateDelegate` :!event `UpdateRightLever`))
  (bind _asbpi_lever_3 (cast `/Game/Blueprint/Actors/BPI_Lever` (`ChildActorComponent.ChildActor` (`self.BP_LeverBucket`))))
  (add `/Game/Blueprint/Actors/BPI_Lever.UpdateLever` _asbpi_lever_3 (`|CreateDelegate` :!event `Update lever axet`))
  (bind _asbpi_lever_4 (cast `/Game/Blueprint/Actors/BPI_Lever` (`ChildActorComponent.ChildActor` (`self.BP_LeverBucket Axes`))))
  (add `/Game/Blueprint/Actors/BPI_Lever.UpdateLever` _asbpi_lever_4 (`|CreateDelegate` :!event `UpdateLeftLever`)))

(event `ButtonEnterPresset`
  (params (ButtonState :type Boolean))
  ;[1 1 1] enter tractor
  (if ButtonState
    (bind _asvrpawn (cast `/Game/Blueprint/Game/VRPawn` (`ActorComponent.GetOwner` (`/Game/Blueprint/Components/BPC_Button.FocusedComponent` (`self.BPC_ButtonEnter`)))))
    (bind _output_get (set `self.VRPawn` _asvrpawn))
    (set `/Game/Blueprint/Game/VRPawn.CanMove` false _output_get)
    (`HeadMountedDisplayFunctionLibrary.ResetOrientationAndPosition` 0.0)
    (`self.K2_AttachToComponent` (`self.VRPawn`) (`self.Arrow`) "None" "SnapToTarget" "SnapToTarget" "KeepWorld" true)
    (`self.K2_SetActorRelativeLocation` (`self.VRPawn`) (0.0 0.0 40.0) false false)))

(event `ButtonExitPresset`
  (params (ButtonState :type Boolean))
  (bind _tractortires (`self.TractorTires`))
  (bind (_returnvalue_x _returnvalue_y) (`KismetMathLibrary.BreakVector` (+ (`SceneComponent.K2_GetComponentLocation` _tractortires) (* (`SceneComponent.GetRightVector` _tractortires) 100.0))))
  ;[1 1 1] Exit Tactor
  (if ButtonState
    (set `/Game/Blueprint/Game/VRPawn.CanMove` true (`self.VRPawn`))
    (`self.K2_DetachFromActor` (`self.VRPawn`) "KeepRelative" "KeepRelative" "KeepRelative")
    (`SceneComponent.K2_AddWorldOffset` (`/Game/Blueprint/Game/VRPawn.DefaultSceneRoot` (`self.VRPawn`)) (`KismetMathLibrary.MakeVector` _returnvalue_x _returnvalue_y) false false)))

(event `UpdateLeftLever`
  (params (LeverAngle :type "Float (double-precision)"))
  ;[1 1 1] SetInput
  (set `self.Left input` (`KismetMathLibrary.MapRangeClamped` LeverAngle 0.0 1.0 1.0 -1.0)))

(event `self.ReceiveTick`
  (params (DeltaSeconds :type "Float (single-precision)"))
  (`|ExecutionSequence`
    (:`then_0`
      (`self.UpdateForce`))
    (:`then_1`
      (`self.DAmping`))
    (:`then_2`
      (`self.UpdateBucketAngle`))))

(event `UpdateRightLever`
  (params (LeverAngle :type "Float (double-precision)"))
  ;[1 1 1] SetInput
  (set `self.Right Input` (`KismetMathLibrary.MapRangeClamped` LeverAngle 0.0 1.0 1.0 -1.0)))

(event `Update lever axet`
  (params (LeverAngle :type "Float (double-precision)"))
  ;[1 1 1] SetInput
  (set `self.AxesBuckettARGETaNGLE` (* LeverAngle 50.0)))

(event `UpdateLeverBucket`
  (params (LeverAngle :type "Float (double-precision)"))
  ;[1 1 1] SetInput
  (set `self.bUCKETtARGETaNGLE` (`KismetMathLibrary.MapRangeClamped` LeverAngle 0.0 1.0 -60.0 30.0)))

(fn `DAmping`
  (bind _tractortires (`self.TractorTires`))
  (`PrimitiveComponent.AddForce` (`self.TractorTires`) (* (`self.GetVelocity`) (`self.GetLinearStopingForce`)) "None" false)
  (`PrimitiveComponent.SetAllPhysicsAngularVelocityInDegrees` (`self.TractorTires`) (`KismetMathLibrary.MakeVector` 0.0 0.0 (`self.GetAngularStopingForce`)) false)
  (bind _returnvalue (`PrimitiveComponent.GetPhysicsLinearVelocity` _tractortires "None"))
  (`PrimitiveComponent.SetPhysicsLinearVelocity` (`self.TractorTires`) (+ _returnvalue (* (`SceneComponent.GetRightVector` (`self.TractorTires`)) (`KismetMathLibrary.Dot_VectorVector` _returnvalue (`SceneComponent.GetRightVector` _tractortires)))) false "None"))

(fn `GetAngularStopingForce`
  (returns (force :type "Float (double-precision)"))
  (bind (_returnvalue_x _returnvalue_y _returnvalue_z) (`KismetMathLibrary.BreakVector` (`PrimitiveComponent.GetPhysicsAngularVelocityInDegrees` (`self.TractorTires`) "None")))
  (return (`KismetMathLibrary.FInterpTo` _returnvalue_z 0.0 (`GameplayStatics.GetWorldDeltaSeconds`) 5.0)))

(fn `GetLinearStopingForce`
  (returns (Force :type "Float (double-precision)"))
  (return (`KismetMathLibrary.MapRangeClamped` (+ (`KismetMathLibrary.Abs` (`self.Left input`)) (`KismetMathLibrary.Abs` (`self.Right Input`))) 0.0 2.0 -400.0 -150.0)))

(fn `UpdateBucketAngle`
  (bind (_relativerotation_roll _relativerotation_pitch) (`KismetMathLibrary.BreakRotator` (`SceneComponent.RelativeRotation` (`self.sm_tracktor_bucket`))))
  (bind (_relativerotation_roll_2 _relativerotation_pitch_2) (`KismetMathLibrary.BreakRotator` (`SceneComponent.RelativeRotation` (`self.sm_tracktor_bucketAxes`))))
  (`SceneComponent.K2_SetRelativeRotation` (`self.sm_tracktor_bucketAxes`) (`KismetMathLibrary.MakeRotator` 0.0 (`KismetMathLibrary.FInterpTo` _relativerotation_pitch_2 (`self.AxesBuckettARGETaNGLE`) (`GameplayStatics.GetWorldDeltaSeconds`) 1.0)) false false)
  (`SceneComponent.K2_SetRelativeRotation` (`self.sm_tracktor_bucket`) (`KismetMathLibrary.MakeRotator` 0.0 (`KismetMathLibrary.FInterpTo` _relativerotation_pitch (`self.bUCKETtARGETaNGLE`) (`GameplayStatics.GetWorldDeltaSeconds`) 1.0)) false false))

(fn `UpdateForce`
  (if (or (> (`KismetMathLibrary.Abs` (`self.Left input`)) (`self.LeversDeadZone`)) (> (`KismetMathLibrary.Abs` (`self.Right Input`)) (`self.LeversDeadZone`)))
    (`|ExecutionSequence`
      (:`then_0`
        (`PrimitiveComponent.AddForceAtLocation` (`self.TractorTires`) (* (`SceneComponent.GetForwardVector` (`self.TractorTires`)) (* (`self.Left input`) (`self.Power`) (`PrimitiveComponent.GetMass` (`self.TractorTires`)))) (`KismetMathLibrary.TransformLocation` (`SceneComponent.K2_GetComponentToWorld` (`self.TractorTires`)) (0.0 -100.0 0.0)) "None"))
      (:`then_1`
        (`PrimitiveComponent.AddForceAtLocation` (`self.TractorTires`) (* (`SceneComponent.GetForwardVector` (`self.TractorTires`)) (* (`self.Right Input`) (`self.Power`) (`PrimitiveComponent.GetMass` (`self.TractorTires`)))) (`KismetMathLibrary.TransformLocation` (`SceneComponent.K2_GetComponentToWorld` (`self.TractorTires`)) (0.0 100.0 0.0)) "None")))))

(fn `UserConstructionScript`)
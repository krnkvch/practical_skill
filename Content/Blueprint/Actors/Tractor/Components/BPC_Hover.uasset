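; BPC_Hover is a hover component for BP_Tractor that pushes the vehicle up from the surface beneath it, acting as a raycast spring-damper suspension point.
; Each tick it traces along its local down axis up to HoverDistance on the Visibility channel, with debug drawing.
; On a hit, it applies force at its location on the tractor's root primitive, combining spring compression with damping from the frame-to-frame change in compression.
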(event `self.ReceiveBeginPlay`
  (bind _asbp_tractor (cast `/Game/Blueprint/Actors/Tractor/BP_Tractor` (`self.GetOwner`)))
  (set `self.BP Tractor` _asbp_tractor))

(event `self.ReceiveTick`
  (params (DeltaSeconds :type "Float (single-precision)"))
  (bind _returnvalue (`self.K2_GetComponentLocation`))
  (`self.BP Tractor`
    (:`then`
      (bind (_outhit _returnvalue_2) (`KismetSystemLibrary.LineTraceSingle` :`Start` _returnvalue :`End` (- _returnvalue (* (`self.GetUpVector`) (`self.HoverDistance`))) :`TraceChannel` "TraceTypeQuery1" :`DrawDebugType` "ForOneFrame"))
      (if _returnvalue_2
        (bind _output_get (set `self.HoverDelta` (- (`self.HoverDistance`) (`.Distance` (`GameplayStatics.BreakHitResult` _outhit)))))
        (`PrimitiveComponent.AddForceAtLocation` (cast `PrimitiveComponent` (`Actor.RootComponent` (`self.BP Tractor`)) :!pure true) (* (`self.GetUpVector`) (+ (* (/ (- _output_get (`self.PreviosDelta`)) (`GameplayStatics.GetWorldDeltaSeconds`)) (`self.DumpingCoefficient`)) (* _output_get (`self.SpringCoefficient`)))) (`self.K2_GetComponentLocation`) "None")
        (set `self.PreviosDelta` (`self.HoverDelta`))))
    (:`else`)))
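; BP_MusicCircle is a Simon-style musical memory game where the player repeats a random sequence of lit, sounding buttons.
; Construction gathers components tagged MusicButton, then a looping timer plays each note by swapping materials before opening input.
; Interact checks the hit button against the expected note, showing green or red with its sound.
; Each completed round generates an entirely new, longer sequence, while a mistake restarts at a short one.
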(event `self.ReceiveBeginPlay`
  (set `self.currentSecuenceLoop` 0)
  (`self.CalculateNotes`)
  (`self.playnotesequence`))

(event `/Game/Blueprint/Game/Interface.Interact`
  (params (`Out HIt` :type "HitResult Structure"))
  (if (`self.isInputMode`)
    (bind (_succes _correct _buttoncomponent _buttonid) (`self.tryPressButton` (`.HitComponent` (`GameplayStatics.BreakHitResult` `Out HIt`))))
    (if _succes
      (`self.interactButton` _correct _buttonid))))

(fn `CalculateNotes`
  (locals (LocalMaxNotes :type Integer :default 0))
  (`KismetArrayLibrary.Array_Clear` (`self.notes`))
  (set `local.LocalMaxNotes` (`self.currentSecuenceLoop`))
  (for _ (range (+ (`local.LocalMaxNotes`) 1))
    (`KismetArrayLibrary.Array_Add` (`self.notes`) (`KismetMathLibrary.RandomInteger` (`self.ButtonCount`))))
  (set `self.sizeofSequence` (`KismetArrayLibrary.Array_Length` (`self.notes`))))

(fn `ClearActivButton`
  (bind _asstatic_mesh_component (cast `StaticMeshComponent` (`|GetArrayItem` (`self.Buttons`) (`self.activButton`))))
  (`PrimitiveComponent.SetMaterial` _asstatic_mesh_component 0 "/Game/Meshes/Materials/M_ColorGray.M_ColorGray"))

(fn `CollectButtons`
  (`KismetArrayLibrary.Array_Clear` (`self.Buttons`))
  (set `self.Buttons` (`self.GetComponentsByTag` "/Script/Engine.ActorComponent" "MusicButton"))
  (set `self.ButtonCount` (`KismetArrayLibrary.Array_Length` (`self.Buttons`))))

(fn `interactButton`
  (params (correct :type Boolean) (buttonID :type Integer))
  (set `self.activButton` buttonID)
  (`KismetSystemLibrary.K2_SetTimer` null "ClearActivButton" (`self.Speed`))
  (`GameplayStatics.PlaySoundAtLocation` (`|GetArrayItem` (`self.sounds`) (`self.activButton`)) (`SceneComponent.K2_GetComponentLocation` (`self.base`)) (struct) 1.0 1.0 0.0 null null null))

(fn `PlayNote`
  (if (< (`self.noteloop`) (`self.sizeofSequence`))
    (set `self.currentNote` (`|GetArrayItem` (`self.notes`) (`self.noteloop`)))
    (if (`self.isTurnOn&`)
      (set `self.isTurnOn&` false)
      (bind _asstatic_mesh_component (cast `StaticMeshComponent` (`|GetArrayItem` (`self.Buttons`) (`self.currentNote`))))
      (`PrimitiveComponent.SetMaterial` _asstatic_mesh_component 0 "/Game/Meshes/Materials/M_ColorGreen.M_ColorGreen")
      (`GameplayStatics.PlaySoundAtLocation` (`|GetArrayItem` (`self.sounds`) (`self.currentNote`)) (`SceneComponent.K2_GetComponentLocation` (`self.base`)) (struct) 1.0 1.0 0.0 null null null)
      (else
        (set `self.isTurnOn&` true)
        (bind _asstatic_mesh_component_2 (cast `StaticMeshComponent` (`|GetArrayItem` (`self.Buttons`) (`self.currentNote`))))
        (`PrimitiveComponent.SetMaterial` _asstatic_mesh_component_2 0 "/Game/Meshes/Materials/M_ColorGray.M_ColorGray")
        (`/Engine/EditorBlueprintResources/StandardMacros.IncrementInt` (`self.noteloop`))))
    (else
      (`KismetSystemLibrary.K2_ClearAndInvalidateTimerHandle` (`self.PlayNoteTimerHandle`))
      (set `self.isInputMode` true)
      (set `self.noteloop` 0))))

(fn `playnotesequence`
  (set `self.isInputMode` false)
  (set `self.noteloop` 0)
  (bind _returnvalue (`KismetSystemLibrary.K2_SetTimer` null "PlayNote" (`self.Speed`) true))
  (set `self.PlayNoteTimerHandle` _returnvalue)
  (`TextRenderComponent.K2_SetText` (`self.TextRender`) (`KismetTextLibrary.Conv_IntToText` (`self.sizeofSequence`))))

(fn `tryPressButton`
  (params (NewParam :type "ActorComponent Object Reference"))
  (returns (succes :type Boolean) (correct :type Boolean) (buttonComponent :type "StaticMeshComponent Object Reference") (buttonID :type Integer))
  (locals (localButton :type "StaticMeshComponent Object Reference") (localButtonID :type Integer :default 0))
  (bind _asstatic_mesh_component (cast `StaticMeshComponent` NewParam)
    (:`then`
      (bind _output_get (set `local.localButton` _asstatic_mesh_component))
      (bind _returnvalue (`KismetArrayLibrary.Array_Find` (`self.Buttons`) _output_get))
      (set `local.localButtonID` _returnvalue)
      (if (== _returnvalue (`|GetArrayItem` (`self.notes`) (`self.noteloop`)))
        (`PrimitiveComponent.SetMaterial` (`local.localButton`) 0 "/Game/Meshes/Materials/M_ColorGreen.M_ColorGreen")
        (`/Engine/EditorBlueprintResources/StandardMacros.IncrementInt` (`self.noteloop`)
          (:`  `
            (if (>= (`self.noteloop`) (`self.sizeofSequence`))
              (`self.updateGameLoop`))
            (return true true (`local.localButton`) (`local.localButtonID`))))
        (else
          (`PrimitiveComponent.SetMaterial` (`local.localButton`) 0 "/Game/Meshes/Materials/M_ColorRed.M_ColorRed")
          (set `self.currentSecuenceLoop` 0)
          (`self.updateGameLoop`)
          (return true false (`local.localButton`) (`local.localButtonID`)))))
    (:`CastFailed`
      (return false false null 0))))

(fn `UpdateBaseColor`
  (`PrimitiveComponent.SetMaterial` (`self.base`) 0 "/Game/Meshes/1-2/Material_017.Material_017"))

(fn `updateGameLoop`
  (`/Engine/EditorBlueprintResources/StandardMacros.IncrementInt` (`self.currentSecuenceLoop`)
    (:`  `
      (`self.CalculateNotes`)
      (`self.playnotesequence`))))

(fn `UserConstructionScript`
  (`self.UpdateBaseColor`)
  (`self.CollectButtons`))
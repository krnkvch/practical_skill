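; TraceObjekt is an interactable actor with a configurable static mesh and text label.
; The construction script applies the Mesh and Text variables to its StaticMesh and TextRender components.
; Activate and Deactivate open and close a Gate on Tick that rotates the mesh a little each frame while open.
; Interact toggles the visibility of the text.
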(event `self.ReceiveTick`
  (params (DeltaSeconds :type "Float (single-precision)"))
  (`/Engine/EditorBlueprintResources/StandardMacros.Gate` true :!label _label
    (:`Exit`
      (`SceneComponent.K2_AddLocalRotation` (`self.StaticMesh`) (struct :`Yaw` 1.0) false false))))

(event `Activate`
  (goto _label :!via `Open`))

(event `Deactivate`
  (goto _label :!via `Close`))

(event `/Game/Blueprint/Game/Interface.Interact`
  (params (`Out HIt` :type "HitResult Structure"))
  (bind _textrender (`self.TextRender`))
  (if (`SceneComponent.bVisible` (`self.TextRender`))
    (`SceneComponent.SetVisibility` _textrender false false)
    (else
      (`SceneComponent.SetVisibility` _textrender true false))))

(fn `UserConstructionScript`
  (`StaticMeshComponent.SetStaticMesh` (`self.StaticMesh`) (`self.Mesh`))
  (`TextRenderComponent.K2_SetText` (`self.TextRender`) (`self.text`)))